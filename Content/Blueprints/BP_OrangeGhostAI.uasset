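; Orange ghost enemy character for a Pac-Man style game that patrols and ends the game when it touches Pac-Man.
; From BeginPlay it walks slowly to random PatrolLocation points via AIMoveTo, pausing briefly before re-calling GuardPatrol on each success, with no failure branch.
; A projectile entering Box only swaps the Sphere to a transparent material; destroy logic is unconnected.
; Pac-Man entering Box1 opens the GameOver level.
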(event OnComponentBeginOverlap(CapsuleComponent)
  (params (OverlappedComponent :type Primitive%20Component%20Object%20Reference) (OtherActor :type Actor%20Object%20Reference) (OtherComp :type Primitive%20Component%20Object%20Reference) (OtherBodyIndex :type Integer) (bFromSweep :type Boolean) (SweepResult :type Hit%20Result%20Structure%20%28by%20ref%29)))

(event OnComponentBeginOverlap(Box)
  (params (OverlappedComponent :type Primitive%20Component%20Object%20Reference) (OtherActor :type Actor%20Object%20Reference) (OtherComp :type Primitive%20Component%20Object%20Reference) (OtherBodyIndex :type Integer) (bFromSweep :type Boolean) (SweepResult :type Hit%20Result%20Structure%20%28by%20ref%29))
  (Utilities|Casting|CastToBP_Projectile OtherActor)
  (Rendering|Material|SetMaterial (Variables|Default|GetSphere) 0 "/Game/Material/mTransparent.mTransparent"))

(event OnComponentBeginOverlap(Box1)
  (params (OverlappedComponent :type Primitive%20Component%20Object%20Reference) (OtherActor :type Actor%20Object%20Reference) (OtherComp :type Primitive%20Component%20Object%20Reference) (OtherBodyIndex :type Integer) (bFromSweep :type Boolean) (SweepResult :type Hit%20Result%20Structure%20%28by%20ref%29))
  (bind _returnvalue (Game|GetPlayerController 0))
  (Utilities|Casting|CastToBP_PacMan OtherActor)
  (Game|OpenLevel(byObjectReference) "/Game/Scenes/GameOver.GameOver")
  (Input|SetInputModeGameOnly _returnvalue false)
  (Variables|/Script/Engine.PlayerController|SetbShowMouseCursor _returnvalue false))

(event Custom|GuardPatrol
  (bind _patrollocation (Variables|Default|GetPatrolLocation))
  ;[1 1 1] Patrol
  (Variables|/Script/Engine.CharacterMovementComponent|SetMaxWalkSpeed (Variables|Character|GetCharacterMovement) 1.5e+02)
  (AI|AIMoveTo self (Utilities|Array|Get(acopy) _patrollocation (Math|Random|RandomInteger (Utilities|Array|Length _patrollocation))) 0 5.0 false
    (:OnSuccess
      (Utilities|FlowControl|Delay (Math|Random|RandomFloatinRange 1.0 3.0))
      (CallFunction|GuardPatrol))))

(event Collision|EventActorBeginOverlap
  (params (OtherActor :type Actor%20Object%20Reference)))

(event EventTick
  (params (DeltaSeconds :type Float%20%28single-precision%29)))

(event EventBeginPlay
  (CallFunction|GuardPatrol))

(fn ConstructionScript)
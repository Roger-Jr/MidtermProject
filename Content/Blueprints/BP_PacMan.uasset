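; BP_PacMan is the player-controlled Pac-Man, handling movement, projectile firing, HUD creation and pause menu input.
; Four input axes add movement along fixed world X/Y directions, and BeginPlay adds missile, score and life widgets to the viewport.
; Firing spends a Missle count to spawn BP_Projectile at ProjectileSpawnLocation, while pause input only adds a PauseMenu widget.
; Box overlap is empty, with ghost-destroy and older projectile nodes left disconnected.
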(event OnComponentBeginOverlap(Box)
  (params (OverlappedComponent :type Primitive%20Component%20Object%20Reference) (OtherActor :type Actor%20Object%20Reference) (OtherComp :type Primitive%20Component%20Object%20Reference) (OtherBodyIndex :type Integer) (bFromSweep :type Boolean) (SweepResult :type Hit%20Result%20Structure%20%28by%20ref%29)))

(event EventBeginPlay
  ;[1 1 1] UI Display
  (bind _returnvalue (UserInterface|CreateWidget "/Game/UI/MissleDisplayWidget.MissleDisplayWidget_C"))
  (bind _returnvalue_2 (UserInterface|CreateWidget "/Game/UI/ScoreDisplayWidget.ScoreDisplayWidget_C"))
  (bind _returnvalue_3 (UserInterface|CreateWidget "/Game/UI/LifeDisplayWidget.LifeDisplayWidget_C"))
  (UserInterface|Viewport|AddtoViewport _returnvalue 0))

(event Collision|EventActorBeginOverlap
  (params (OtherActor :type Actor%20Object%20Reference)))

(event EventTick
  (params (DeltaSeconds :type Float%20%28single-precision%29)))

(event Input|ActionEvents|InputActionFireProjectile
  (params (Key :type Key%20Structure :default "None"))
  ;[1 1 1] New Mechanic/Projectile
  (:Pressed
    (if (>= (Variables|Default|GetMissle) 1)
      (Game|SpawnActorfromClass "/Game/Blueprints/BP_Projectile.BP_Projectile_C" (Transformation|GetWorldTransform (Variables|Default|GetProjectileSpawnLocation)) "AlwaysSpawn" "MultiplyWithRoot" 0 0)
      (Variables|Default|SetMissle (- (Variables|Default|GetMissle) 1)))))

(event Input|ActionEvents|InputActionPauseInput
  (params (Key :type Key%20Structure :default "None"))
  ;[1 1 1] Pause Input
  (:Pressed
    (bind _returnvalue (UserInterface|CreateWidget "/Game/UI/PauseMenu.PauseMenu_C" (Game|GetPlayerController 0)))
    (UserInterface|Viewport|AddtoViewport _returnvalue 0)))

(event Input|AxisEvents|InputAxisMoveForward
  (params (AxisValue :type Float%20%28single-precision%29))
  ;[1 1 1] Movement
  (Pawn|Input|AddMovementInput "0.000000,0.500000,0.000000" AxisValue false))

(event Input|AxisEvents|InputAxisMoveBackward
  (params (AxisValue :type Float%20%28single-precision%29))
  ;[1 1 1] Movement
  (Pawn|Input|AddMovementInput "0.000000,-0.500000,0.000000" AxisValue false))

(event Input|AxisEvents|InputAxisMoveRight
  (params (AxisValue :type Float%20%28single-precision%29))
  ;[1 1 1] Movement
  (Pawn|Input|AddMovementInput "-0.500000,0.000000,0.000000" AxisValue false))

(event Input|AxisEvents|InputAxisMoveLeft
  (params (AxisValue :type Float%20%28single-precision%29))
  ;[1 1 1] Movement
  (Pawn|Input|AddMovementInput "0.500000,0.000000,0.000000" AxisValue false))

(fn ConstructionScript)
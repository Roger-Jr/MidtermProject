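; Pac-Man game mode that shows a pause display widget at startup and holds basic scoring logic.
; BeginPlay creates the PauseDisplayWidget and adds it to the viewport.
; AddScore sets CurrentScore from its input plus a separate ScoreAdd variable, printing a win message when the result is zero.
; A BP_Pellet counting chain is unconnected and never runs, and Tick is disabled.
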(event EventBeginPlay
  (bind _returnvalue (UserInterface|CreateWidget "/Game/UI/PauseDisplayWidget.PauseDisplayWidget_C"))
  (UserInterface|Viewport|AddtoViewport _returnvalue 0))

(event EventTick
  (params (DeltaSeconds :type Float%20%28single-precision%29)))

(fn ConstructionScript)

(fn AddScore
  (params (ScoreToAdd :type Integer))
  (bind _output_get (Variables|Default|SetCurrentScore (+ ScoreToAdd (Variables|Default|GetScoreAdd))))
  (if (== _output_get 0)
    (Development|PrintString "YouWin!")))
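; Test AI pawn for a ghost, meant to wander to random points inside its WanderingArea box.
; BeginPlay sets a looping timer for WanderRandomly but targets the FloatingPawnMovement component, although the function is defined on this Blueprint.
; WanderRandomly sends the AI controller to a random point in the box via SimpleMoveToLocation and prints a debug string.
; Actor overlap casts to BP_Projectile with no follow-up logic, and Tick is empty.
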(event EventBeginPlay
  (Utilities|Time|SetTimerbyFunctionName (Variables|Default|GetFloatingPawnMovement) "WanderRandomly" 5.0 true))

(event Collision|EventActorBeginOverlap
  (params (OtherActor :type Actor%20Object%20Reference))
  (Utilities|Casting|CastToBP_Projectile OtherActor))

(event EventTick
  (params (DeltaSeconds :type Float%20%28single-precision%29)))

(fn ConstructionScript)

(fn WanderRandomly
  (bind _wanderingarea (Variables|Default|GetWanderingArea))
  (AI|Navigation|SimpleMovetoLocation (AI|GetAIController 0) (Math|Random|RandomPointinBoundingBox (Transformation|GetWorldLocation _wanderingarea) (Components|Box|GetScaledBoxExtent _wanderingarea)))
  (Development|PrintString "Point"))
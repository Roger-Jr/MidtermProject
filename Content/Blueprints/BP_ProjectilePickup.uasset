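; BP_ProjectilePickup is a Pac-Man pickup that grants the player a missile and 100 score.
; On any actor overlap it updates player character 0's BP_PacMan without checking the overlapping actor, then destroys itself.
; It also counts as a pellet, decrementing TotalPellets on PacManGameMode.
; When that count reaches zero, it opens the Victory level with game-only input and a hidden cursor.
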(event EventBeginPlay)

(event Collision|EventActorBeginOverlap
  (params (OtherActor :type Actor%20Object%20Reference))
  (bind _returnvalue (Game|GetPlayerController 0))
  (bind _asbp_pac_man (Utilities|Casting|CastToBP_PacMan (Game|GetPlayerCharacter 0)))
  (Variables|/Game/Blueprints/BP_PacMan.BP_PacMan_C|SetMissle _asbp_pac_man (+ (Variables|/Game/Blueprints/BP_PacMan.BP_PacMan_C|GetMissle _asbp_pac_man) 1))
  (Variables|/Game/Blueprints/BP_PacMan.BP_PacMan_C|SetScore _asbp_pac_man (+ (Variables|/Game/Blueprints/BP_PacMan.BP_PacMan_C|GetScore _asbp_pac_man) 100))
  (bind _aspac_man_game_mode (Utilities|Casting|CastToPacManGameMode (Game|GetGameMode)))
  (bind _output_get (Variables|/Game/Blueprints/PacManGameMode.PacManGameMode_C|SetTotalPellets _aspac_man_game_mode (- (Variables|/Game/Blueprints/PacManGameMode.PacManGameMode_C|GetTotalPellets _aspac_man_game_mode) 1)))
  (Actor|DestroyActor)
  (if (== _output_get 0)
    (Game|OpenLevel(byObjectReference) "/Game/Scenes/Victory.Victory")
    (Input|SetInputModeGameOnly _returnvalue false)
    (Variables|/Script/Engine.PlayerController|SetbShowMouseCursor _returnvalue false)))

(event EventTick
  (params (DeltaSeconds :type Float%20%28single-precision%29)))

(fn ConstructionScript)